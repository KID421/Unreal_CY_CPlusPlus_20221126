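; Triangular pyramid actor (BP_三角錐) that continuously bobs up and down between its starting height and a set offset above it.
; BeginPlay records the start Z as the minimum, adds the offset for the maximum, and starts upward.
; Tick moves Z by speed scaled with DeltaSeconds, keeping X and Y, and flips a direction boolean after passing either limit, without clamping.
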(event EventBeginPlay
  (bind _returnvalue (Transformation|GetActorLocation))
  (bind _output_get (Variables|Default|Set當前高度 (.z _returnvalue))) ; 0
  (Variables|Default|Set最小高度 _output_get) ; 0
  (Variables|Default|Set最大高度 (+ (.z _returnvalue) (Variables|Default|Get往上位移的高度))) ; 200
  (Variables|Default|Set是否往上 true) ; 往上：是
)

(event EventTick
  (params (DeltaSeconds :type Float%20%28single-precision%29))
  (bind _returnvalue (Transformation|GetActorLocation))
  (bind _移動速度 (Variables|Default|Get移動速度))
  (bind _returnvalue_2 (* DeltaSeconds _移動速度))
  (if (Variables|Default|Get是否往上) ; 判斷式 if
    (Variables|Default|Set當前高度 (+ (Variables|Default|Get當前高度) _returnvalue_2)) ; 100
    (else
      (Variables|Default|Set當前高度 (- (Variables|Default|Get當前高度) _returnvalue_2)) ; 100
    ))
  (Transformation|SetActorLocation (Math|Vector|MakeVector (.x _returnvalue) (.y _returnvalue) (Variables|Default|Get當前高度)) false false) ; 設定物件座標
  (if (> (Variables|Default|Get當前高度) (Variables|Default|Get最大高度)) ; 如果高度大於最大高度
    (Variables|Default|Set是否往上 false) ; 就往下
    (elif (< (Variables|Default|Get當前高度) (Variables|Default|Get最小高度)) ; 如果高度小於最小高度
      (Variables|Default|Set是否往上 true) ; 就往上
    )))

(fn ConstructionScript)